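; BP_Color is a clickable cube actor that changes color with each click and eventually explodes.
; BeginPlay creates a dynamic material instance, and each click increments the red channel of its Basecolor parameter.
; Each click also plays a sound at a rising pitch, which doubles as the counter: past a threshold, the actor plays an eject sound, spawns the Boom particle system and destroys itself.
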(event `self.ReceiveBeginPlay`
  (bind _returnvalue (`PrimitiveComponent.CreateDynamicMaterialInstance` (`self.Cube`) 0 null "None"))
  (set `self.Material Instance` _returnvalue)
  (set `self.Add` 0.0))

(event `self.Cube.OnClicked`
  (params (TouchedComponent :type "PrimitiveComponent Object Reference") (ButtonPressed :type "Key Structure"))
  (bind _output_get (set `self.Add` (+ (`self.Add`) (`self.Plus`))))
  (`MaterialInstanceDynamic.SetVectorParameterValue` (`self.Material Instance`) "Basecolor" (make `LinearColor` _output_get 0.0 0.0 1.0))
  (bind _output_get_2 (set `self.PitchAdd` (+ (`self.PitchAdd`) 0.2)))
  (`GameplayStatics.PlaySound2D` "/Engine/VREditor/Sounds/UI/Click_on_Button.Click_on_Button" 10.0 _output_get_2 0.0 null null)
  (if (> _output_get_2 2.0)
    (`GameplayStatics.PlaySound2D` "/Engine/EditorSounds/GamePreview/EjectFromPlayer.EjectFromPlayer" 5.0 1.0 0.0 null null)
    (`NiagaraFunctionLibrary.SpawnSystemAtLocation` "/Game/Effect/Boom.Boom" (`self.K2_GetActorLocation`))
    (`self.K2_DestroyActor`)))

(fn `UserConstructionScript`)